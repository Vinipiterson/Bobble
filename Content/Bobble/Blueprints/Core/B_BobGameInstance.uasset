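; Game instance for Bobble that holds per-level data and persists best times to the "Bob" save slot.
; On Init it loads LevelDatas from an existing save, then flags IsReady, which is also set when no save exists.
; SaveLevel finds a level by internal name, keeps the lower time (zero counts as unset), and always writes a fresh save object.
; Levels missing from the array are not added.
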(event `self.ReceiveInit`
  (bind _returnvalue (`GameplayStatics.DoesSaveGameExist` "Bob"))
  (if _returnvalue
    (bind _returnvalue_2 (`GameplayStatics.LoadGameFromSlot` "Bob"))
    (bind _asb_bob_save_game (cast `/Game/Bobble/Blueprints/Core/B_BobSaveGame` _returnvalue_2))
    (set `self.LevelDatas` (`/Game/Bobble/Blueprints/Core/B_BobSaveGame.LevelDatas` _asb_bob_save_game))
    (set `self.bIsReady` true)
    (else
      (set `self.bIsReady` true))))

(fn `FindLevel`
  (params (InternalName :type String))
  (returns (LevelData :type "/Game/Bobble/Blueprints/Data/S_LevelData Structure") (Index :type Integer))
  (for (_array_element _array_index) (`self.LevelDatas`)
    (if (`KismetStringLibrary.EqualEqual_StrStr` InternalName (`.InternalName_13_868E1D5F4ADC74302BC920B67C984AC9` (break `/Game/Bobble/Blueprints/Data/S_LevelData` _array_element)))
      (return _array_element _array_index)))
  (return (struct) -1))

(fn `SaveLevel`
  (params (LevelName :type String) (Time :type "Float (double-precision)"))
  (bind (_leveldata _index) (`self.FindLevel` LevelName))
  (bind ((`BestTime_11_74EEEB9946F7DC4616EC609127F2C0DB` _besttime)) (break `/Game/Bobble/Blueprints/Data/S_LevelData` _leveldata))
  (`|ExecutionSequence`
    (:`then_0`
      (if (!= _index -1)
        (if (or (< (`local.Time`) _besttime) (== _besttime 0.0))
          (bind _structout (setmembers `/Game/Bobble/Blueprints/Data/S_LevelData` :`StructRef` _leveldata :`BestTime` (`local.Time`)))
          (`KismetArrayLibrary.Array_Set` (`self.LevelDatas`) _index _structout true))))
    (:`then_1`
      (bind _returnvalue (`GameplayStatics.CreateSaveGameObject` "/Game/Bobble/Blueprints/Core/B_BobSaveGame.B_BobSaveGame_C"))
      (set `/Game/Bobble/Blueprints/Core/B_BobSaveGame.LevelDatas` (`self.LevelDatas`) _returnvalue)
      (`GameplayStatics.SaveGameToSlot` _returnvalue "Bob"))))