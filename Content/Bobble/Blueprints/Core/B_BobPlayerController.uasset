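; Player controller for Bobble that owns the HUD overlay, the level timer and pausing.
; On begin play it adds the Enhanced Input mapping context and creates the character overlay widget.
; Tick advances the time while the timer runs and pushes it to the overlay, which also receives notifications and level-finish results.
; Pause and focus toggles switch input mode and mouse cursor visibility.
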(event `self.ReceiveBeginPlay`
  (`self.Input`)
  (`self.UI`)
  (set `self.CurrentTime` 0.0))

(event `/Game/Bobble/Blueprints/B_PCInterface.Notify`
  (params (Message :type Text))
  (`/Game/Bobble/Blueprints/UI/UI_CharacterOverlay.AddNotify` (`self.CharacterOverlay`) Message))

(event `self.ReceiveTick`
  (params (DeltaSeconds :type "Float (single-precision)"))
  (if (`self.IsTimerRunning`)
    (`self.SetCurrentTime` (+ (`self.CurrentTime`) DeltaSeconds))))

(event `/Game/Bobble/Blueprints/B_PCInterface.StopTimer`
  (set `self.IsTimerRunning` false))

(event `/Game/Bobble/Blueprints/B_PCInterface.ToggleFocus`
  (params (UI :type Boolean))
  (if UI
    (`WidgetBlueprintLibrary.SetInputMode_UIOnlyEx` self (`self.CharacterOverlay`))
    (set `self.bShowMouseCursor` true)
    (else
      (`WidgetBlueprintLibrary.SetInputMode_GameOnly` self)
      (set `self.bShowMouseCursor` false))))

(event `/Game/Bobble/Blueprints/B_PCInterface.OnFinishLevel`
  (params (LevelData :type "/Game/Bobble/Blueprints/Data/S_LevelData Structure") (Time :type "Float (double-precision)"))
  (`/Game/Bobble/Blueprints/B_PCInterface.OnFinishLevel` (`self.CharacterOverlay`) LevelData Time))

(event `EnhancedInput|/Game/Bobble/Input/Actions/IA_Pause`
  (params (ActionValue :type Boolean) (ElapsedSeconds :type "Float (double-precision)") (TriggeredSeconds :type "Float (double-precision)") (InputAction :type "InputAction Object Reference" :default "/Game/Bobble/Input/Actions/IA_Pause.IA_Pause"))
  (:`Triggered`
    (`self.TogglePause`)))

(event `/Game/Bobble/Blueprints/B_PCInterface.UpdatePause`
  (`self.TogglePause`))

(fn `GetCurrentTime`
  (returns (Time :type "Float (double-precision)"))
  (return (`self.CurrentTime`)))

(fn `Input`
  (message `EnhancedInputSubsystemInterface.AddMappingContext` (subsystem `EnhancedInputLocalPlayerSubsystem`) "/Game/Bobble/Input/IMC_Bob.IMC_Bob" 0 (struct)))

(fn `SetCurrentTime`
  (params (NewTime :type "Float (double-precision)"))
  (bind _output_get (set `self.CurrentTime` NewTime))
  (bind _characteroverlay (`self.CharacterOverlay`)
    (:`then`
      (message `/Game/Bobble/Blueprints/B_PCInterface.OnTimeSet` _characteroverlay _output_get))
    (:`else`)))

(fn `TogglePause`
  (if (`GameplayStatics.IsGamePaused`)
    (`GameplayStatics.SetGamePaused` false)
    (`/Game/Bobble/Blueprints/UI/UI_CharacterOverlay.TogglePause` (`self.CharacterOverlay`))
    (`WidgetBlueprintLibrary.SetInputMode_GameOnly` self)
    (set `self.bShowMouseCursor` false)
    (else
      (`GameplayStatics.SetGamePaused` true)
      (`/Game/Bobble/Blueprints/UI/UI_CharacterOverlay.TogglePause` (`self.CharacterOverlay`))
      (`WidgetBlueprintLibrary.SetInputMode_GameAndUIEx` self (`self.CharacterOverlay`))
      (set `self.bShowMouseCursor` true))))

(fn `UI`
  (bind _returnvalue (`|CreateWidget` "/Game/Bobble/Blueprints/UI/UI_CharacterOverlay.UI_CharacterOverlay_C" self))
  (bind _output_get (set `self.CharacterOverlay` _returnvalue))
  (`UserWidget.AddToViewport` _output_get 0))

(fn `UserConstructionScript`)