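; B_VenomBoblle is a damaging bubble hazard that can travel along a spline.
; When spline following is enabled, Tick advances a distance along the path and teleport-free, unswept moves place the actor there.
; Closed splines restart at the end, while open ones ping-pong by flipping a direction multiplier at each endpoint.
; Overlapping its sphere applies damage, then briefly disables sphere collision as a hit cooldown.
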(event `self.ReceiveTick`
  (params (DeltaSeconds :type "Float (single-precision)"))
  (`self.UpdateLocation` DeltaSeconds))

(event `self.Sphere.OnComponentBeginOverlap`
  (params (OverlappedComponent :type "PrimitiveComponent Object Reference") (OtherActor :type "Actor Object Reference") (OtherComp :type "PrimitiveComponent Object Reference") (OtherBodyIndex :type Integer) (bFromSweep :type Boolean) (SweepResult :type "HitResult Structure (by ref)"))
  (`GameplayStatics.ApplyDamage` OtherActor 1.0)
  (`PrimitiveComponent.SetCollisionEnabled` (`self.Sphere`) "NoCollision")
  (`KismetSystemLibrary.Delay` 2.0)
  (`PrimitiveComponent.SetCollisionEnabled` (`self.Sphere`) "QueryOnly"))

(fn `UpdateLocation`
  (params (`Delta Time` :type "Float (double-precision)"))
  (bind _spline (`self.Spline`))
  (if (`self.ShouldFollowSpline`)
    (bind _output_get (set `self.CurrentDistance` (+ (`self.CurrentDistance`) (* (`self.Speed`) `Delta Time` (`self.DistanceMultiplier`)))))
    (bind _returnvalue (`SplineComponent.GetLocationAtDistanceAlongSpline` (`self.Spline`) _output_get "World"))
    (`self.K2_SetActorLocation` _returnvalue)
    (if (== _returnvalue (`SplineComponent.GetLocationAtSplinePoint` _spline (- (`SplineComponent.GetNumberOfSplinePoints` _spline) 1) "World"))
      (if (`SplineComponent.IsClosedLoop` (`self.Spline`))
        (set `self.CurrentDistance` 0.0)
        (else
          (set `self.DistanceMultiplier` -1.0)))
      (elif (== (`SceneComponent.K2_GetComponentLocation` (`self.Sphere`)) (`SplineComponent.GetLocationAtSplinePoint` (`self.Spline`) 0 "World") :`ErrorTolerance` 1.0)
        (set `self.CurrentDistance` 0.0)
        (set `self.DistanceMultiplier` 1.0)))))

(fn `UserConstructionScript`)