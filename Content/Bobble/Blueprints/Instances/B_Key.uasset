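; B_Key is a key pickup that the player collects by overlapping it.
; On overlap with player character 0, it counts all B_Key actors in the level, including itself, to detect the last key.
; The last key plays an unlock sound and any other plays a collect sound, then the key destroys itself.
; The Blueprint holds no unlock logic beyond that sound.
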(event `self.ReceiveActorBeginOverlap`
  (params (OtherActor :type "Actor Object Reference"))
  (if (== OtherActor (`GameplayStatics.GetPlayerCharacter` 0))
    (bind _outactors (`GameplayStatics.GetAllActorsOfClass` "B_Key_C"))
    (if (== (`KismetArrayLibrary.Array_Length` _outactors) 1)
      (`GameplayStatics.PlaySoundAtLocation` (`self.UnlockSound`) (`self.K2_GetActorLocation`) (struct) 2.0 1.0 0.0 null null null null)
      (else
        (`GameplayStatics.PlaySoundAtLocation` (`self.CollectSound`) (`self.K2_GetActorLocation`) (struct) 1.0 1.0 0.0 null null null null)))
    (`self.K2_DestroyActor`)))

(fn `UserConstructionScript`)