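; B_Door is a locked door that opens on overlap once no B_Key actors remain in the level.
; While keys remain, overlap sends the player controller a message with the count still needed and plays a closed sound.
; Otherwise OpenDoor plays an unlock sound, disables the Box collision and plays the MoveDoor timeline, whose update lerps RotationRoot's yaw through a quarter turn.
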(event `self.ReceiveActorBeginOverlap`
  (params (OtherActor :type "Actor Object Reference"))
  (bind _outactors (`GameplayStatics.GetAllActorsOfClass` "/Game/Bobble/Blueprints/Instances/B_Key.B_Key_C"))
  (bind _returnvalue (`KismetArrayLibrary.Array_Length` _outactors))
  (if (> _returnvalue 0)
    (message `/Game/Bobble/Blueprints/B_PCInterface.Notify` (`GameplayStatics.GetPlayerController` 0) (`|FormatText` "You need {num} more keys" _returnvalue))
    (`GameplayStatics.PlaySound2D` "/Game/Bobble/Assets/Sounds/S_DoorClosed.S_DoorClosed" 0.2 1.0 0.0 null null)
    (else
      (`self.Open Door`))))

(event `Open Door`
  (`GameplayStatics.PlaySound2D` "/Game/Bobble/Assets/Sounds/S_UnlockDoor.S_UnlockDoor" 0.2 1.0 0.0 null null)
  (`PrimitiveComponent.SetCollisionEnabled` (`self.Box`) "NoCollision")
  (`TimelineComponent.PlayFromStart` (`self.MoveDoor`)))

(fn `UserConstructionScript`)