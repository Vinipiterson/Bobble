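; B_LevelEnd is the level finish trigger that records the player's time and ends the run.
; When its Box is overlapped, it gets the current time from the player controller and saves it under the level name in B_BobGameInstance.
; It then toggles controller focus, passes the level data and time to the controller's finish message, and disables the player's movement.
; The overlapping actor is not checked.
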(event `self.Box.OnComponentBeginOverlap`
  (params (OverlappedComponent :type "PrimitiveComponent Object Reference") (OtherActor :type "Actor Object Reference") (OtherComp :type "PrimitiveComponent Object Reference") (OtherBodyIndex :type Integer) (bFromSweep :type Boolean) (SweepResult :type "HitResult Structure (by ref)"))
  (bind _charactermovement (`Character.CharacterMovement` (`GameplayStatics.GetPlayerCharacter` 0)))
  (bind _time (message `/Game/Bobble/Blueprints/B_PCInterface.GetCurrentTime` (`GameplayStatics.GetPlayerController` 0)))
  (bind _asb_bob_game_instance (cast `/Game/Bobble/Blueprints/Core/B_BobGameInstance` (`GameplayStatics.GetGameInstance`)))
  (bind _returnvalue (`GameplayStatics.GetCurrentLevelName` true))
  (`/Game/Bobble/Blueprints/Core/B_BobGameInstance.SaveLevel` _asb_bob_game_instance _returnvalue _time)
  (message `/Game/Bobble/Blueprints/B_PCInterface.ToggleFocus` (`GameplayStatics.GetPlayerController` 0) true)
  (message `/Game/Bobble/Blueprints/B_PCInterface.OnFinishLevel` (`GameplayStatics.GetPlayerController` 0) (`/Game/Bobble/Blueprints/Core/B_BobGameInstance.FindLevel` _asb_bob_game_instance _returnvalue) _time)
  (`MovementComponent.StopMovementImmediately` _charactermovement)
  (`CharacterMovementComponent.DisableMovement` _charactermovement))

(fn `UserConstructionScript`)