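; B_BobCharacter is the player character, handling movement input and death.
; IA_Move adds movement along fixed world right and forward axes.
; When HealthComponent fires Die, it enables post-processing, turns the static mesh into a physics body, disables damage and input, stops the controller's timer message, then restarts the level after a short delay.
; Pressing 1 destroys every B_Key actor in the level.
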(event `EnhancedInput|/Game/Bobble/Input/Actions/IA_Move`
  (params (ActionValue :type "Vector2D Structure") (ElapsedSeconds :type "Float (double-precision)") (TriggeredSeconds :type "Float (double-precision)") (InputAction :type "InputAction Object Reference" :default "/Game/Bobble/Input/Actions/IA_Move.IA_Move"))
  (:`Triggered`
    (`self.AddMovementInput` (`KismetMathLibrary.Vector_Right`) ActionValue_X)
    (`self.AddMovementInput` (`KismetMathLibrary.Vector_Forward`) ActionValue_Y)))

(event `self.HealthComponent.Die`
  (bind _returnvalue (`GameplayStatics.GetPlayerController` 0))
  (set `PostProcessComponent.bEnabled` true (`self.PostProcess`))
  (`PrimitiveComponent.SetCollisionEnabled` (`self.StaticMesh`) "PhysicsOnly")
  (set `self.bCanBeDamaged` false)
  (`PrimitiveComponent.SetSimulatePhysics` (`self.StaticMesh`) true)
  (`self.DisableInput` _returnvalue)
  (message `/Game/Bobble/Blueprints/B_PCInterface.StopTimer` _returnvalue)
  (`KismetSystemLibrary.Delay` 3.0)
  (`KismetSystemLibrary.ExecuteConsoleCommand` "RestartLevel" null))

(event `Key|One`
  (params (Key :type "Key Structure"))
  (:`Pressed`
    (bind _outactors (`GameplayStatics.GetAllActorsOfClass` "/Game/Bobble/Blueprints/Instances/B_Key.B_Key_C"))
    (for _array_element _outactors
      (`self.K2_DestroyActor` _array_element))))

(fn `UserConstructionScript`)