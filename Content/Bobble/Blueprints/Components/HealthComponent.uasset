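; HealthComponent is an actor component that tracks integer health for its owner and signals when that owner dies.
; On BeginPlay it fills health to the maximum, binds to the owner's OnTakeAnyDamage and broadcasts OnHealthUpdated.
; The Damage handler subtracts truncated damage without clamping, broadcasts OnHealthUpdated with the previous health value, and calls Die whenever health is below one.
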(event `self.ReceiveBeginPlay`
  (set `self.CurrentHealth` (`self.MaxHealth`))
  (add `Actor.OnTakeAnyDamage` (`self.GetOwner`) (`|CreateDelegate` :!event `Damage`))
  (`self.OnHealthUpdated` (`self.CurrentHealth`)))

(fn `Damage`
  (params (DamagedActor :type "Actor Object Reference") (Damage :type "Float (single-precision)") (DamageType :type "DamageType Object Reference") (InstigatedBy :type "Controller Object Reference") (DamageCauser :type "Actor Object Reference"))
  (locals (OldHealth :type Integer))
  (set `local.OldHealth` (`self.CurrentHealth`))
  (set `self.CurrentHealth` (`KismetMathLibrary.Conv_Int64ToInt` (- (`self.CurrentHealth`) (`KismetMathLibrary.Conv_DoubleToInt64` Damage))))
  (`self.OnHealthUpdated` (`local.OldHealth`))
  (if (< (`self.CurrentHealth`) 1)
    (`self.Die`)))